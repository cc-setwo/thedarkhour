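; Menu camera Blueprint that sets up the main menu when play begins.
; BeginPlay creates the MainMenu widget, shows the mouse cursor and starts a held camera fade that partially tints the view behind the menu.
; The widget's first button is bound to a custom event that opens the Start level.
; The camera's initial field of view is stored but not used in these graphs.
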(event `self.ReceiveBeginPlay`
  (bind _returnvalue (`GameplayStatics.GetPlayerController` 0))
  (`GameplayStatics.GetPlayerControllerID` (`GameplayStatics.GetPlayerController` 0))
  (bind _returnvalue_2 (`|CreateWidget` "/Game/FirstPersonBP/Blueprints/MainMenu.MainMenu_C"))
  (`UserWidget.AddToViewport` _returnvalue_2 0)
  (add `Button.OnClicked` (`/Game/FirstPersonBP/Blueprints/MainMenu.Button_0` _returnvalue_2) (delegate `CustomEvent_0`))
  (set `PlayerController.bShowMouseCursor` true _returnvalue)
  (`PlayerCameraManager.StartCameraFade` :`self` (`GameplayStatics.GetPlayerCameraManager` _returnvalue) :`ToAlpha` 0.45 :`Duration` 3.0 :`bHoldWhenFinished` true)
  (set `self.InitialFieldOfView` (`CameraComponent.FieldOfView` (`self.CameraComponent`))))

(event `CustomEvent_0`
  (`GameplayStatics.OpenLevel` "Start"))

(fn `UserConstructionScript`)